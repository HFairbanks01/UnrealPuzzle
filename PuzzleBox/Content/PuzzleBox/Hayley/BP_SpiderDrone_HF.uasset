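; BP_SpiderDrone_HF is a spider drone pawn that chases the player character, reissuing AI MoveTo every second from BeginPlay.
; Pawn sensing issues another move toward BP_Person and immediately calls Dead, which sets spider flags and destroys the drone after a short delay.
; Each tick tries copying those flags from BP_HoverDrone_HF, but casts a spider drone instance to that class.
; The capsule overlap only casts to BP_Person, with no further action.
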(event `self.ReceiveBeginPlay`
  (`self.Chase`))

(event `self.ReceiveTick`
  (params (DeltaSeconds :type "Float (single-precision)"))
  (`self.CheckHoverSpider`))

(event `Chase`
  ;[1 1 1] Chases the player
  (`|AIMoveTo` self (0.0 0.0 0.0) (`GameplayStatics.GetPlayerCharacter` 0)
    (:`then`
      (`KismetSystemLibrary.Delay` 1.0)
      (`self.Chase`))))

(event `self.PawnSensing.OnSeePawn`
  (params (Pawn :type "Pawn Object Reference"))
  ;[1 1 1] Moves to Player
  (bind _asbp_person (cast `/Game/PuzzleBox/Core/BP_Person` (`GameplayStatics.GetPlayerCharacter` 0)))
  (`|AIMoveTo` self (0.0 0.0 0.0) _asbp_person
    (:`then`
      (`KismetSystemLibrary.PrintString` "Sees player")
      (`self.Dead`))))

(event `self.CapsuleComponent.OnComponentBeginOverlap`
  (params (OverlappedComponent :type "PrimitiveComponent Object Reference") (OtherActor :type "Actor Object Reference") (OtherComp :type "PrimitiveComponent Object Reference") (OtherBodyIndex :type Integer) (bFromSweep :type Boolean) (SweepResult :type "HitResult Structure (by ref)"))
  (cast `/Game/PuzzleBox/Core/BP_Person` OtherActor))

(event `Dead`
  (set `self.SpiderS` false)
  (set `self.SpiderDestroy` true)
  (`KismetSystemLibrary.Delay` 0.5)
  (`self.K2_DestroyActor`)
  (`KismetSystemLibrary.PrintString` "PawnDestroyed"))

(fn `CheckHoverSpider`
  (bind _outactors (`GameplayStatics.GetAllActorsOfClass` "BP_SpiderDrone_HF_C"))
  (bind _output_get (set `self.SpiderReference` (`|GetArrayItem` _outactors)))
  (bind _asbp_hover_drone_hf (cast `/Game/PuzzleBox/Hayley/BP_HoverDrone_HF` _output_get))
  (set `self.SpiderS` (`/Game/PuzzleBox/Hayley/BP_HoverDrone_HF.Spiders` _asbp_hover_drone_hf))
  (set `self.SpiderDestroy` (`/Game/PuzzleBox/Hayley/BP_HoverDrone_HF.SpiderDestroyed` _asbp_hover_drone_hf)))

(fn `UserConstructionScript`)