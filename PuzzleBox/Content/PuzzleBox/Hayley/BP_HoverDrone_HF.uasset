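; Hover drone AI pawn that roams randomly, chases characters it sees and spawns spider and bomb drones.
; Tick starts delayed wander moves to random reachable points within a radius, gated by a Move flag, while PawnSensing triggers pursuit.
; It spawns a spider after BeginPlay, and each finished or failed wander picks between further spawns and status checks.
; CheckSpider and CheckBomb copy alive and destroyed flags from the last spawned drones to drive that choice.
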(event `self.ReceiveBeginPlay`
  (`KismetSystemLibrary.Delay` 5.0)
  (`self.SpawnSpiders`)
  (set `self.Destroy` false)
  (set `self.SpiderDestroyed` false)
  (`self.CheckSpider`)
  (`self.CheckBomb`))

(event `self.ReceiveTick`
  (params (DeltaSeconds :type "Float (single-precision)"))
  ;[1 1 1] Smart AI
  (`KismetSystemLibrary.Delay` 2.0)
  (if (not (`self.Move`))
    (set `self.Move` true)
    (`|AIMoveTo` self (`NavigationSystemV1.K2_GetRandomReachablePointInRadius` (`self.K2_GetActorLocation`) 1000.0 null null) null
      (:`OnSuccess`
        _)
      (:`OnFail`
        _))
    (set `self.Move` false)
    (if (`self.SpiderDestroyed`)
      (`self.SpawnBombs`)
      (elif (`self.Spiders`)
        (`self.CheckSpider`)
        (`self.CheckBomb`)
        (elif (`self.Destroy`)
          (`self.SpawnSpiders`)
          (elif (`self.Bombs`)
            (`self.CheckSpider`)
            (`self.CheckBomb`)
            (else
              (`self.SpawnBombs`))))))))

(event `SpawnSpiders`
  ;[1 1 1] Spawn Enemies
  (`KismetSystemLibrary.Delay` 5.0)
  (bind _returnvalue (`AIBlueprintHelperLibrary.SpawnAIFromClass` "/Game/PuzzleBox/Hayley/BP_SpiderDrone_HF.BP_SpiderDrone_HF_C" null (`SceneComponent.K2_GetComponentLocation` (`self.Spawn`))))
  (set `self.SpiderRef` _returnvalue)
  (`KismetSystemLibrary.PrintString` "SpiderSpawn")
  (set `self.Spiders` true))

(event `SpawnBombs`
  ;[1 1 1] Spawn Enemies
  (`KismetSystemLibrary.Delay` 10.0)
  (bind _returnvalue (`AIBlueprintHelperLibrary.SpawnAIFromClass` "/Game/PuzzleBox/Hayley/BP_BombDrone_HF.BP_BombDrone_HF_C" null (`SceneComponent.K2_GetComponentLocation` (`self.Spawn`))))
  (set `self.BombRef` _returnvalue)
  (`KismetSystemLibrary.PrintString` "BombSpawn")
  (set `self.Bombs` true))

(event `self.PawnSensing.OnSeePawn`
  (params (Pawn :type "Pawn Object Reference"))
  ;[1 1 1] Sees Player
  (bind _ascharacter (cast `Character` Pawn))
  (set `self.Move` true)
  (`|AIMoveTo` self (0.0 0.0 0.0) _ascharacter
    (:`OnSuccess`
      _)
    (:`OnFail`
      _))
  (`KismetSystemLibrary.Delay` 0.5)
  (set `self.Move` false))

(fn `CheckBomb`
  (bind _asbp_bomb_drone_hf (cast `/Game/PuzzleBox/Hayley/BP_BombDrone_HF` (`self.BombRef`)))
  (set `self.Bombs` (`/Game/PuzzleBox/Hayley/BP_BombDrone_HF.BombS` _asbp_bomb_drone_hf))
  (set `self.Destroy` (`/Game/PuzzleBox/Hayley/BP_BombDrone_HF.BombDestroy` _asbp_bomb_drone_hf)))

(fn `CheckSpider`
  (bind _asbp_spider_drone_hf (cast `/Game/PuzzleBox/Hayley/BP_SpiderDrone_HF` (`self.SpiderRef`)))
  (set `self.Spiders` (`/Game/PuzzleBox/Hayley/BP_SpiderDrone_HF.SpiderS` _asbp_spider_drone_hf))
  (set `self.SpiderDestroyed` (`/Game/PuzzleBox/Hayley/BP_SpiderDrone_HF.SpiderDestroy` _asbp_spider_drone_hf)))

(fn `UserConstructionScript`)