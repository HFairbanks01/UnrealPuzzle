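; Trigger actor for a push-block puzzle that locks BP_PushBlock_DK blocks in place when they enter one of three trigger boxes.
; Each box's overlap event checks its own Overlapping flag, casts to the block, disables its physics and increments the shared Align counter.
; The flag then clears so that box counts only once, and debug prints show the count.
; Nothing here acts on the Align total.
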(event `self.TriggerBox1.OnComponentBeginOverlap`
  (params (OverlappedComponent :type "PrimitiveComponent Object Reference") (OtherActor :type "Actor Object Reference") (OtherComp :type "PrimitiveComponent Object Reference") (OtherBodyIndex :type Integer) (bFromSweep :type Boolean) (SweepResult :type "HitResult Structure (by ref)"))
  (if (`self.Overlapping3`)
    (bind _asbp_push_block_dk (cast `/Game/PuzzleBox/DavidKingsley/Core/BP_PushBlock_DK` OtherActor))
    (`PrimitiveComponent.SetSimulatePhysics` (`/Game/PuzzleBox/DavidKingsley/Core/BP_PushBlock_DK.PushBlock` _asbp_push_block_dk) false)
    (bind _output_get (set `self.Align` (+ (`self.Align`) 1)))
    (`KismetSystemLibrary.PrintString` "Set")
    (`KismetSystemLibrary.PrintString` (`KismetStringLibrary.Conv_IntToString` _output_get))
    (set `self.Overlapping3` false)))

(event `self.TriggerBox2.OnComponentBeginOverlap`
  (params (OverlappedComponent :type "PrimitiveComponent Object Reference") (OtherActor :type "Actor Object Reference") (OtherComp :type "PrimitiveComponent Object Reference") (OtherBodyIndex :type Integer) (bFromSweep :type Boolean) (SweepResult :type "HitResult Structure (by ref)"))
  (if (`self.Overlapping1`)
    (bind _asbp_push_block_dk (cast `/Game/PuzzleBox/DavidKingsley/Core/BP_PushBlock_DK` OtherActor))
    (`PrimitiveComponent.SetSimulatePhysics` (`/Game/PuzzleBox/DavidKingsley/Core/BP_PushBlock_DK.PushBlock` _asbp_push_block_dk) false)
    (bind _output_get (set `self.Align` (+ (`self.Align`) 1)))
    (`KismetSystemLibrary.PrintString` "Set")
    (`KismetSystemLibrary.PrintString` (`KismetStringLibrary.Conv_IntToString` _output_get))
    (set `self.Overlapping1` false)))

(event `self.TriggerBox3.OnComponentBeginOverlap`
  (params (OverlappedComponent :type "PrimitiveComponent Object Reference") (OtherActor :type "Actor Object Reference") (OtherComp :type "PrimitiveComponent Object Reference") (OtherBodyIndex :type Integer) (bFromSweep :type Boolean) (SweepResult :type "HitResult Structure (by ref)"))
  (if (`self.Overlapping2`)
    (bind _asbp_push_block_dk (cast `/Game/PuzzleBox/DavidKingsley/Core/BP_PushBlock_DK` OtherActor))
    (`PrimitiveComponent.SetSimulatePhysics` (`/Game/PuzzleBox/DavidKingsley/Core/BP_PushBlock_DK.PushBlock` _asbp_push_block_dk) false)
    (bind _output_get (set `self.Align` (+ (`self.Align`) 1)))
    (`KismetSystemLibrary.PrintString` "Set")
    (`KismetSystemLibrary.PrintString` (`KismetStringLibrary.Conv_IntToString` _output_get))
    (set `self.Overlapping2` false)))

(fn `UserConstructionScript`)