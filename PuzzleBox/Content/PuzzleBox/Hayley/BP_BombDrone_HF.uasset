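; Bomb drone pawn that chases the player and destroys itself once it reaches a player it has seen.
; BeginPlay starts an AIMoveTo loop toward the player, while PawnSensing triggers a move that ends in Dead.
; Dead sets bomb flags, then destroys the actor after a short delay.
; Each Tick, CheckHoverBomb casts the first BP_BombDrone_HF found to BP_HoverDrone_HF to copy its bomb flags.
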(event `self.ReceiveBeginPlay`
  (`self.Chase`))

(event `self.ReceiveTick`
  (params (DeltaSeconds :type "Float (single-precision)"))
  (`self.CheckHoverBomb`))

(event `Chase`
  ;[1 1 1] Directly chases player
  (`|AIMoveTo` self (0.0 0.0 0.0) (`GameplayStatics.GetPlayerCharacter` 0)
    (:`then`
      (`KismetSystemLibrary.Delay` 1.0)
      (`self.Chase`))))

(event `self.PawnSensing.OnSeePawn`
  (params (Pawn :type "Pawn Object Reference"))
  ;[1 1 1] Moves to Player
  (bind _asbp_person (cast `/Game/PuzzleBox/Core/BP_Person` (`GameplayStatics.GetPlayerCharacter` 0)))
  (`|AIMoveTo` self (0.0 0.0 0.0) _asbp_person
    (:`then`
      (`KismetSystemLibrary.PrintString` "Sees Player")
      (`self.Dead`))))

(event `Dead`
  (set `self.BombS` false)
  (set `self.BombDestroy` true)
  (`KismetSystemLibrary.Delay` 0.5)
  (`self.K2_DestroyActor`)
  (`KismetSystemLibrary.PrintString` "PawnDestroyed"))

(fn `CheckHoverBomb`
  (bind _outactors (`GameplayStatics.GetAllActorsOfClass` "BP_BombDrone_HF_C"))
  (bind _output_get (set `self.BombReference` (`|GetArrayItem` _outactors)))
  (bind _asbp_hover_drone_hf (cast `/Game/PuzzleBox/Hayley/BP_HoverDrone_HF` _output_get))
  (set `self.BombS` (`/Game/PuzzleBox/Hayley/BP_HoverDrone_HF.Bombs` _asbp_hover_drone_hf))
  (set `self.BombDestroy` (`/Game/PuzzleBox/Hayley/BP_HoverDrone_HF.Destroy` _asbp_hover_drone_hf)))

(fn `UserConstructionScript`)