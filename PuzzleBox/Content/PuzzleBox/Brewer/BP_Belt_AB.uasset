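; Conveyor belt actor in the PuzzleBox Brewer content that carries along whatever actors rest in its trigger volume.
; While OnOff is true, Tick offsets every actor overlapping Box along the forward vector of Cube, scaled by Speed and delta time.
; Movement is a direct world offset without sweep, so it ignores collision along the path.
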(event `self.ReceiveTick`
  (params (DeltaSeconds :type "Float (single-precision)"))
  (if (`self.OnOff`)
    (for _array_element (`PrimitiveComponent.GetOverlappingActors` (`self.Box`) null)
      (`self.K2_AddActorWorldOffset` _array_element (* (`KismetMathLibrary.GetForwardVector` (`SceneComponent.K2_GetComponentRotation` (`self.Cube`))) (* DeltaSeconds (`self.Speed`))) false false))))

(fn `UserConstructionScript`)