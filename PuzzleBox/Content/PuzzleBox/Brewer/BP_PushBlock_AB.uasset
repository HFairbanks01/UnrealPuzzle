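; Pushable puzzle block that only responds to physics while the player character is next to it.
; Overlap with either the X_Box or Y_Box trigger by BP_Person_DK turns on physics simulation on the PushBlock mesh, and leaving turns it off.
; Both triggers toggle the same simulation flag; the graph itself applies no axis constraint or push force.
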(event `self.Y_Box.OnComponentBeginOverlap`
  (params (OverlappedComponent :type "PrimitiveComponent Object Reference") (OtherActor :type "Actor Object Reference") (OtherComp :type "PrimitiveComponent Object Reference") (OtherBodyIndex :type Integer) (bFromSweep :type Boolean) (SweepResult :type "HitResult Structure (by ref)"))
  ;[1 1 1] Move Box on Y Axis
  (cast `/Game/PuzzleBox/DavidKingsley/Core/BP_Person_DK` OtherActor)
  (`PrimitiveComponent.SetSimulatePhysics` (`self.PushBlock`) true))

(event `self.Y_Box.OnComponentEndOverlap`
  (params (OverlappedComponent :type "PrimitiveComponent Object Reference") (OtherActor :type "Actor Object Reference") (OtherComp :type "PrimitiveComponent Object Reference") (OtherBodyIndex :type Integer))
  ;[1 1 1] Move Box on Y Axis
  (cast `/Game/PuzzleBox/DavidKingsley/Core/BP_Person_DK` OtherActor)
  (`PrimitiveComponent.SetSimulatePhysics` (`self.PushBlock`) false))

(event `self.X_Box.OnComponentBeginOverlap`
  (params (OverlappedComponent :type "PrimitiveComponent Object Reference") (OtherActor :type "Actor Object Reference") (OtherComp :type "PrimitiveComponent Object Reference") (OtherBodyIndex :type Integer) (bFromSweep :type Boolean) (SweepResult :type "HitResult Structure (by ref)"))
  ;[1 1 1] Move Box on X Axis
  (cast `/Game/PuzzleBox/DavidKingsley/Core/BP_Person_DK` OtherActor)
  (`PrimitiveComponent.SetSimulatePhysics` (`self.PushBlock`) true))

(event `self.X_Box.OnComponentEndOverlap`
  (params (OverlappedComponent :type "PrimitiveComponent Object Reference") (OtherActor :type "Actor Object Reference") (OtherComp :type "PrimitiveComponent Object Reference") (OtherBodyIndex :type Integer))
  ;[1 1 1] Move Box on X Axis
  (cast `/Game/PuzzleBox/DavidKingsley/Core/BP_Person_DK` OtherActor)
  (`PrimitiveComponent.SetSimulatePhysics` (`self.PushBlock`) false))

(fn `UserConstructionScript`)