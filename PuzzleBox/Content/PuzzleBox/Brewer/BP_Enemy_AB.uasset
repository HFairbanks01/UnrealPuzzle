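; Enemy actor for a puzzle game that wanders in random directions, destroys any BP_Person_AB it overlaps and is destroyed by BP_PushBlock_AB.
; Tick moves it along the Cube's forward vector at Speed without sweeping.
; A one-second Delay in Tick periodically snaps Cube and Box to one of four right-angle yaws.
; Nested random rolls choose that heading, so the odds are uneven.
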(event `self.ReceiveActorBeginOverlap`
  (params (OtherActor :type "Actor Object Reference"))
  (if (== (`GameplayStatics.GetObjectClass` OtherActor) "/Game/PuzzleBox/Brewer/BP_PushBlock_AB.BP_PushBlock_AB_C")
    (`self.K2_DestroyActor`)
    (elif (== (`GameplayStatics.GetObjectClass` OtherActor) "/Game/PuzzleBox/Brewer/BP_Person_AB.BP_Person_AB_C")
      (`self.K2_DestroyActor` OtherActor))))

(event `self.ReceiveTick`
  (params (DeltaSeconds :type "Float (single-precision)"))
  (bind _returnvalue (`KismetMathLibrary.RandomIntegerInRange` 0 3))
  (bind _cube (`self.Cube`))
  (`self.K2_AddActorWorldOffset` (* (`KismetMathLibrary.GetForwardVector` (`SceneComponent.K2_GetComponentRotation` (`self.Cube`))) (* DeltaSeconds (`self.Speed`))))
  (`KismetSystemLibrary.Delay` 1.0)
  (`/Engine/EditorBlueprintResources/StandardMacros.CompareInt` _returnvalue 1
    (:`>`
      (`/Engine/EditorBlueprintResources/StandardMacros.CompareInt` _returnvalue 3
        (:`==`
          (`SceneComponent.K2_SetWorldRotation` _cube (struct :`Yaw` 270.0) false false)
          (`SceneComponent.K2_SetWorldRotation` (`self.Box`) (struct :`Yaw` 270.0) false false))
        (:`<`
          (`SceneComponent.K2_SetWorldRotation` _cube (struct :`Yaw` 180.0) false false)
          (`SceneComponent.K2_SetWorldRotation` (`self.Box`) (struct :`Yaw` 180.0) false false))))
    (:`==`
      (`SceneComponent.K2_SetWorldRotation` _cube (struct :`Yaw` 90.0) false false)
      (`SceneComponent.K2_SetWorldRotation` (`self.Box`) (struct :`Yaw` 90.0) false false))
    (:`<`
      (`SceneComponent.K2_SetWorldRotation` (`self.Box`) (struct) false false)
      (`SceneComponent.K2_SetWorldRotation` _cube (struct) false false))))

(fn `UserConstructionScript`)