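; BP_Enemy1_DK is a turret-like enemy that turns toward and shoots at characters it sees.
; On each PawnSensing sighting it snaps its rotation to face the character, then spawns a half-scale BP_Bullet_DK at ProjectileSpawnLocation.
; An impulse along the Cube's forward vector launches the bullet, scaled by ShootForce.
; The SpawnProjectile flag and a delay gate the fire rate.
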(event `self.PawnSensing.OnSeePawn`
  (params (Pawn :type "Pawn Object Reference"))
  (bind (_returnvalue_location _returnvalue_rotation) (`KismetMathLibrary.BreakTransform` (`SceneComponent.K2_GetComponentToWorld` (`self.ProjectileSpawnLocation`))))
  ;[1 1 1] Player Targeting Enemy
  (bind _ascharacter (cast `Character` Pawn))
  (`|ExecutionSequence`
    (:`then_0`
      (`self.K2_SetActorRotation` (`KismetMathLibrary.FindLookAtRotation` (`self.K2_GetActorLocation`) (`self.K2_GetActorLocation` _ascharacter))))
    (:`then_1`
      (if (`self.SpawnProjectile`)
        (bind _returnvalue (`|SpawnActorFromClass` "/Game/PuzzleBox/DavidKingsley/Core/BP_Bullet_DK.BP_Bullet_DK_C" (`KismetMathLibrary.MakeTransform` _returnvalue_location _returnvalue_rotation (0.5 0.5 0.5)) "Undefined" "OverrideRootScale" null null))
        (`PrimitiveComponent.AddImpulse` (`/Game/PuzzleBox/DavidKingsley/Core/BP_Bullet_DK.Sphere` _returnvalue) (* (`SceneComponent.GetForwardVector` (`self.Cube`)) (`self.ShootForce`)) "None" false)
        (set `self.SpawnProjectile` false)
        (`KismetSystemLibrary.Delay` 10.0)
        (set `self.SpawnProjectile` true)))))

(fn `UserConstructionScript`)