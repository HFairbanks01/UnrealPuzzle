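; BP_Enemy2_DK is a stationary-style shooter enemy that fires bullets when its PawnSensing component sees a pawn.
; On sight, it spawns a half-scale BP_Bullet_DK at the ProjectileSpawnLocation and pushes it with an impulse along the Cube's forward vector scaled by ShootForce.
; A SpawnProjectile flag and a five-second delay act as the cooldown between shots.
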(event `self.PawnSensing.OnSeePawn`
  (params (Pawn :type "Pawn Object Reference"))
  (bind (_returnvalue_location _returnvalue_rotation) (`KismetMathLibrary.BreakTransform` (`SceneComponent.K2_GetComponentToWorld` (`self.ProjectileSpawnLocation`))))
  ;[1 1 1] Target Player Enemy
  (if (`self.SpawnProjectile`)
    (bind _returnvalue (`|SpawnActorFromClass` "/Game/PuzzleBox/DavidKingsley/Core/BP_Bullet_DK.BP_Bullet_DK_C" (`KismetMathLibrary.MakeTransform` _returnvalue_location _returnvalue_rotation (0.5 0.5 0.5)) "Undefined" "OverrideRootScale" null null))
    (`PrimitiveComponent.AddImpulseAtLocation` (`/Game/PuzzleBox/DavidKingsley/Core/BP_Bullet_DK.Sphere` _returnvalue) (* (`SceneComponent.GetForwardVector` (`self.Cube`)) (`self.ShootForce`)) (0.0 0.0 0.0) "None")
    (set `self.SpawnProjectile` false)
    (`KismetSystemLibrary.Delay` 5.0)
    (set `self.SpawnProjectile` true)))

(fn `UserConstructionScript`)