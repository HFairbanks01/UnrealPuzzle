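; Push-block puzzle actor whose 19 trigger boxes detect BP_PushBlock_DK actors and count how many are in place.
; Each box has its own one-shot flag; an overlapping block stops simulating physics, increments the shared Align counter and prints debug text.
; The overlap logic is duplicated per box, and the hand-off of Align to BP_FinalDoor_DK's FinalAllign is unconnected, so it never runs.
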(event `self.TriggerBox1.OnComponentBeginOverlap`
  (params (OverlappedComponent :type "PrimitiveComponent Object Reference") (OtherActor :type "Actor Object Reference") (OtherComp :type "PrimitiveComponent Object Reference") (OtherBodyIndex :type Integer) (bFromSweep :type Boolean) (SweepResult :type "HitResult Structure (by ref)"))
  ;[1 1 1] Trigger Box/ Counter 1
  (if (`self.Overlapping1`)
    (bind _asbp_push_block_dk (cast `/Game/PuzzleBox/DavidKingsley/Core/BP_PushBlock_DK` OtherActor))
    (`PrimitiveComponent.SetSimulatePhysics` (`/Game/PuzzleBox/DavidKingsley/Core/BP_PushBlock_DK.PushBlock` _asbp_push_block_dk) false)
    (bind _output_get (set `self.Align` (+ (`self.Align`) 1)))
    (`KismetSystemLibrary.PrintString` "Set")
    (`KismetSystemLibrary.PrintString` (`KismetStringLibrary.Conv_IntToString` _output_get))
    (set `self.Overlapping1` false)))

(event `self.TriggerBox2.OnComponentBeginOverlap`
  (params (OverlappedComponent :type "PrimitiveComponent Object Reference") (OtherActor :type "Actor Object Reference") (OtherComp :type "PrimitiveComponent Object Reference") (OtherBodyIndex :type Integer) (bFromSweep :type Boolean) (SweepResult :type "HitResult Structure (by ref)"))
  ;[1 1 1] Trigger Box/ Counter 2
  (if (`self.Overlapping2`)
    (bind _asbp_push_block_dk (cast `/Game/PuzzleBox/DavidKingsley/Core/BP_PushBlock_DK` OtherActor))
    (`PrimitiveComponent.SetSimulatePhysics` (`/Game/PuzzleBox/DavidKingsley/Core/BP_PushBlock_DK.PushBlock` _asbp_push_block_dk) false)
    (bind _output_get (set `self.Align` (+ (`self.Align`) 1)))
    (`KismetSystemLibrary.PrintString` "Set")
    (`KismetSystemLibrary.PrintString` (`KismetStringLibrary.Conv_IntToString` _output_get))
    (set `self.Overlapping2` false)))

(event `self.TriggerBox3.OnComponentBeginOverlap`
  (params (OverlappedComponent :type "PrimitiveComponent Object Reference") (OtherActor :type "Actor Object Reference") (OtherComp :type "PrimitiveComponent Object Reference") (OtherBodyIndex :type Integer) (bFromSweep :type Boolean) (SweepResult :type "HitResult Structure (by ref)"))
  ;[1 1 1] TriggerBox/ Counter 3
  (if (`self.Overlapping3`)
    (bind _asbp_push_block_dk (cast `/Game/PuzzleBox/DavidKingsley/Core/BP_PushBlock_DK` OtherActor))
    (`PrimitiveComponent.SetSimulatePhysics` (`/Game/PuzzleBox/DavidKingsley/Core/BP_PushBlock_DK.PushBlock` _asbp_push_block_dk) false)
    (bind _output_get (set `self.Align` (+ (`self.Align`) 1)))
    (`KismetSystemLibrary.PrintString` "Set")
    (`KismetSystemLibrary.PrintString` (`KismetStringLibrary.Conv_IntToString` _output_get))
    (set `self.Overlapping3` false)))

(event `self.TriggerBox5.OnComponentBeginOverlap`
  (params (OverlappedComponent :type "PrimitiveComponent Object Reference") (OtherActor :type "Actor Object Reference") (OtherComp :type "PrimitiveComponent Object Reference") (OtherBodyIndex :type Integer) (bFromSweep :type Boolean) (SweepResult :type "HitResult Structure (by ref)"))
  ;[1 1 1] Box Trigger/ Counter 5
  (if (`self.Overlapping5`)
    (bind _asbp_push_block_dk (cast `/Game/PuzzleBox/DavidKingsley/Core/BP_PushBlock_DK` OtherActor))
    (`PrimitiveComponent.SetSimulatePhysics` (`/Game/PuzzleBox/DavidKingsley/Core/BP_PushBlock_DK.PushBlock` _asbp_push_block_dk) false)
    (bind _output_get (set `self.Align` (+ (`self.Align`) 1)))
    (`KismetSystemLibrary.PrintString` "Set")
    (`KismetSystemLibrary.PrintString` (`KismetStringLibrary.Conv_IntToString` _output_get))
    (set `self.Overlapping5` false)))

(event `self.TriggerBox6.OnComponentBeginOverlap`
  (params (OverlappedComponent :type "PrimitiveComponent Object Reference") (OtherActor :type "Actor Object Reference") (OtherComp :type "PrimitiveComponent Object Reference") (OtherBodyIndex :type Integer) (bFromSweep :type Boolean) (SweepResult :type "HitResult Structure (by ref)"))
  ;[1 1 1] Box Trigger/ Counter 6
  (if (`self.Overlapping6`)
    (bind _asbp_push_block_dk (cast `/Game/PuzzleBox/DavidKingsley/Core/BP_PushBlock_DK` OtherActor))
    (`PrimitiveComponent.SetSimulatePhysics` (`/Game/PuzzleBox/DavidKingsley/Core/BP_PushBlock_DK.PushBlock` _asbp_push_block_dk) false)
    (bind _output_get (set `self.Align` (+ (`self.Align`) 1)))
    (`KismetSystemLibrary.PrintString` "Set")
    (`KismetSystemLibrary.PrintString` (`KismetStringLibrary.Conv_IntToString` _output_get))
    (set `self.Overlapping6` false)))

(event `self.TriggerBox7.OnComponentBeginOverlap`
  (params (OverlappedComponent :type "PrimitiveComponent Object Reference") (OtherActor :type "Actor Object Reference") (OtherComp :type "PrimitiveComponent Object Reference") (OtherBodyIndex :type Integer) (bFromSweep :type Boolean) (SweepResult :type "HitResult Structure (by ref)"))
  ;[1 1 1] Box Trigger/ Counter 7
  (if (`self.Overlapping7`)
    (bind _asbp_push_block_dk (cast `/Game/PuzzleBox/DavidKingsley/Core/BP_PushBlock_DK` OtherActor))
    (`PrimitiveComponent.SetSimulatePhysics` (`/Game/PuzzleBox/DavidKingsley/Core/BP_PushBlock_DK.PushBlock` _asbp_push_block_dk) false)
    (bind _output_get (set `self.Align` (+ (`self.Align`) 1)))
    (`KismetSystemLibrary.PrintString` "Set")
    (`KismetSystemLibrary.PrintString` (`KismetStringLibrary.Conv_IntToString` _output_get))
    (set `self.Overlapping7` false)))

(event `self.TriggerBox8.OnComponentBeginOverlap`
  (params (OverlappedComponent :type "PrimitiveComponent Object Reference") (OtherActor :type "Actor Object Reference") (OtherComp :type "PrimitiveComponent Object Reference") (OtherBodyIndex :type Integer) (bFromSweep :type Boolean) (SweepResult :type "HitResult Structure (by ref)"))
  ;[1 1 1] Box Trigger/ Counter 8
  (if (`self.Overlapping8`)
    (bind _asbp_push_block_dk (cast `/Game/PuzzleBox/DavidKingsley/Core/BP_PushBlock_DK` OtherActor))
    (`PrimitiveComponent.SetSimulatePhysics` (`/Game/PuzzleBox/DavidKingsley/Core/BP_PushBlock_DK.PushBlock` _asbp_push_block_dk) false)
    (bind _output_get (set `self.Align` (+ (`self.Align`) 1)))
    (`KismetSystemLibrary.PrintString` "Set")
    (`KismetSystemLibrary.PrintString` (`KismetStringLibrary.Conv_IntToString` _output_get))
    (set `self.Overlapping8` false)))

(event `self.TriggerBox9.OnComponentBeginOverlap`
  (params (OverlappedComponent :type "PrimitiveComponent Object Reference") (OtherActor :type "Actor Object Reference") (OtherComp :type "PrimitiveComponent Object Reference") (OtherBodyIndex :type Integer) (bFromSweep :type Boolean) (SweepResult :type "HitResult Structure (by ref)"))
  ;[1 1 1] Box Trigger/ Counter 9
  (if (`self.Overlapping9`)
    (bind _asbp_push_block_dk (cast `/Game/PuzzleBox/DavidKingsley/Core/BP_PushBlock_DK` OtherActor))
    (`PrimitiveComponent.SetSimulatePhysics` (`/Game/PuzzleBox/DavidKingsley/Core/BP_PushBlock_DK.PushBlock` _asbp_push_block_dk) false)
    (bind _output_get (set `self.Align` (+ (`self.Align`) 1)))
    (`KismetSystemLibrary.PrintString` "Set")
    (`KismetSystemLibrary.PrintString` (`KismetStringLibrary.Conv_IntToString` _output_get))
    (set `self.Overlapping9` false)))

(event `self.TriggerBox10.OnComponentBeginOverlap`
  (params (OverlappedComponent :type "PrimitiveComponent Object Reference") (OtherActor :type "Actor Object Reference") (OtherComp :type "PrimitiveComponent Object Reference") (OtherBodyIndex :type Integer) (bFromSweep :type Boolean) (SweepResult :type "HitResult Structure (by ref)"))
  ;[1 1 1] Box Trigger/ Counter 10
  (if (`self.Overlapping10`)
    (bind _asbp_push_block_dk (cast `/Game/PuzzleBox/DavidKingsley/Core/BP_PushBlock_DK` OtherActor))
    (`PrimitiveComponent.SetSimulatePhysics` (`/Game/PuzzleBox/DavidKingsley/Core/BP_PushBlock_DK.PushBlock` _asbp_push_block_dk) false)
    (bind _output_get (set `self.Align` (+ (`self.Align`) 1)))
    (`KismetSystemLibrary.PrintString` "Set")
    (`KismetSystemLibrary.PrintString` (`KismetStringLibrary.Conv_IntToString` _output_get))
    (set `self.Overlapping10` false)))

(event `self.TriggerBox11.OnComponentBeginOverlap`
  (params (OverlappedComponent :type "PrimitiveComponent Object Reference") (OtherActor :type "Actor Object Reference") (OtherComp :type "PrimitiveComponent Object Reference") (OtherBodyIndex :type Integer) (bFromSweep :type Boolean) (SweepResult :type "HitResult Structure (by ref)"))
  ;[1 1 1] Box Trigger/ Counter 11
  (if (`self.Overlapping11`)
    (bind _asbp_push_block_dk (cast `/Game/PuzzleBox/DavidKingsley/Core/BP_PushBlock_DK` OtherActor))
    (`PrimitiveComponent.SetSimulatePhysics` (`/Game/PuzzleBox/DavidKingsley/Core/BP_PushBlock_DK.PushBlock` _asbp_push_block_dk) false)
    (bind _output_get (set `self.Align` (+ (`self.Align`) 1)))
    (`KismetSystemLibrary.PrintString` "Set")
    (`KismetSystemLibrary.PrintString` (`KismetStringLibrary.Conv_IntToString` _output_get))
    (set `self.Overlapping11` false)))

(event `self.TriggerBox12.OnComponentBeginOverlap`
  (params (OverlappedComponent :type "PrimitiveComponent Object Reference") (OtherActor :type "Actor Object Reference") (OtherComp :type "PrimitiveComponent Object Reference") (OtherBodyIndex :type Integer) (bFromSweep :type Boolean) (SweepResult :type "HitResult Structure (by ref)"))
  ;[1 1 1] Box Trigger/ Counter 12
  (if (`self.Overlapping12`)
    (bind _asbp_push_block_dk (cast `/Game/PuzzleBox/DavidKingsley/Core/BP_PushBlock_DK` OtherActor))
    (`PrimitiveComponent.SetSimulatePhysics` (`/Game/PuzzleBox/DavidKingsley/Core/BP_PushBlock_DK.PushBlock` _asbp_push_block_dk) false)
    (bind _output_get (set `self.Align` (+ (`self.Align`) 1)))
    (`KismetSystemLibrary.PrintString` "Set")
    (`KismetSystemLibrary.PrintString` (`KismetStringLibrary.Conv_IntToString` _output_get))
    (set `self.Overlapping12` false)))

(event `self.TriggerBox13.OnComponentBeginOverlap`
  (params (OverlappedComponent :type "PrimitiveComponent Object Reference") (OtherActor :type "Actor Object Reference") (OtherComp :type "PrimitiveComponent Object Reference") (OtherBodyIndex :type Integer) (bFromSweep :type Boolean) (SweepResult :type "HitResult Structure (by ref)"))
  ;[1 1 1] Box Trigger/ Counter 13
  (if (`self.Overlapping13`)
    (bind _asbp_push_block_dk (cast `/Game/PuzzleBox/DavidKingsley/Core/BP_PushBlock_DK` OtherActor))
    (`PrimitiveComponent.SetSimulatePhysics` (`/Game/PuzzleBox/DavidKingsley/Core/BP_PushBlock_DK.PushBlock` _asbp_push_block_dk) false)
    (bind _output_get (set `self.Align` (+ (`self.Align`) 1)))
    (`KismetSystemLibrary.PrintString` "Set")
    (`KismetSystemLibrary.PrintString` (`KismetStringLibrary.Conv_IntToString` _output_get))
    (set `self.Overlapping13` false)))

(event `self.TriggerBox14.OnComponentBeginOverlap`
  (params (OverlappedComponent :type "PrimitiveComponent Object Reference") (OtherActor :type "Actor Object Reference") (OtherComp :type "PrimitiveComponent Object Reference") (OtherBodyIndex :type Integer) (bFromSweep :type Boolean) (SweepResult :type "HitResult Structure (by ref)"))
  ;[1 1 1] Box Trigger/ Counter 14
  (if (`self.Overlapping14`)
    (bind _asbp_push_block_dk (cast `/Game/PuzzleBox/DavidKingsley/Core/BP_PushBlock_DK` OtherActor))
    (`PrimitiveComponent.SetSimulatePhysics` (`/Game/PuzzleBox/DavidKingsley/Core/BP_PushBlock_DK.PushBlock` _asbp_push_block_dk) false)
    (bind _output_get (set `self.Align` (+ (`self.Align`) 1)))
    (`KismetSystemLibrary.PrintString` "Set")
    (`KismetSystemLibrary.PrintString` (`KismetStringLibrary.Conv_IntToString` _output_get))
    (set `self.Overlapping14` false)))

(event `self.TriggerBox15.OnComponentBeginOverlap`
  (params (OverlappedComponent :type "PrimitiveComponent Object Reference") (OtherActor :type "Actor Object Reference") (OtherComp :type "PrimitiveComponent Object Reference") (OtherBodyIndex :type Integer) (bFromSweep :type Boolean) (SweepResult :type "HitResult Structure (by ref)"))
  ;[1 1 1] Box Trigger/ Counter 15
  (if (`self.Overlapping15`)
    (bind _asbp_push_block_dk (cast `/Game/PuzzleBox/DavidKingsley/Core/BP_PushBlock_DK` OtherActor))
    (`PrimitiveComponent.SetSimulatePhysics` (`/Game/PuzzleBox/DavidKingsley/Core/BP_PushBlock_DK.PushBlock` _asbp_push_block_dk) false)
    (bind _output_get (set `self.Align` (+ (`self.Align`) 1)))
    (`KismetSystemLibrary.PrintString` "Set")
    (`KismetSystemLibrary.PrintString` (`KismetStringLibrary.Conv_IntToString` _output_get))
    (set `self.Overlapping15` false)))

(event `self.TriggerBox16.OnComponentBeginOverlap`
  (params (OverlappedComponent :type "PrimitiveComponent Object Reference") (OtherActor :type "Actor Object Reference") (OtherComp :type "PrimitiveComponent Object Reference") (OtherBodyIndex :type Integer) (bFromSweep :type Boolean) (SweepResult :type "HitResult Structure (by ref)"))
  ;[1 1 1] Box Trigger/ Counter 16
  (if (`self.Overlapping16`)
    (bind _asbp_push_block_dk (cast `/Game/PuzzleBox/DavidKingsley/Core/BP_PushBlock_DK` OtherActor))
    (`PrimitiveComponent.SetSimulatePhysics` (`/Game/PuzzleBox/DavidKingsley/Core/BP_PushBlock_DK.PushBlock` _asbp_push_block_dk) false)
    (bind _output_get (set `self.Align` (+ (`self.Align`) 1)))
    (`KismetSystemLibrary.PrintString` "Set")
    (`KismetSystemLibrary.PrintString` (`KismetStringLibrary.Conv_IntToString` _output_get))
    (set `self.Overlapping16` false)))

(event `self.TriggerBox17.OnComponentBeginOverlap`
  (params (OverlappedComponent :type "PrimitiveComponent Object Reference") (OtherActor :type "Actor Object Reference") (OtherComp :type "PrimitiveComponent Object Reference") (OtherBodyIndex :type Integer) (bFromSweep :type Boolean) (SweepResult :type "HitResult Structure (by ref)"))
  ;[1 1 1] Box Trigger/ Counter 17
  (if (`self.Overlapping17`)
    (bind _asbp_push_block_dk (cast `/Game/PuzzleBox/DavidKingsley/Core/BP_PushBlock_DK` OtherActor))
    (`PrimitiveComponent.SetSimulatePhysics` (`/Game/PuzzleBox/DavidKingsley/Core/BP_PushBlock_DK.PushBlock` _asbp_push_block_dk) false)
    (bind _output_get (set `self.Align` (+ (`self.Align`) 1)))
    (`KismetSystemLibrary.PrintString` "Set")
    (`KismetSystemLibrary.PrintString` (`KismetStringLibrary.Conv_IntToString` _output_get))
    (set `self.Overlapping17` false)))

(event `self.TriggerBox18.OnComponentBeginOverlap`
  (params (OverlappedComponent :type "PrimitiveComponent Object Reference") (OtherActor :type "Actor Object Reference") (OtherComp :type "PrimitiveComponent Object Reference") (OtherBodyIndex :type Integer) (bFromSweep :type Boolean) (SweepResult :type "HitResult Structure (by ref)"))
  ;[1 1 1] Box Trigger/ Counter 18
  (if (`self.Overlapping18`)
    (bind _asbp_push_block_dk (cast `/Game/PuzzleBox/DavidKingsley/Core/BP_PushBlock_DK` OtherActor))
    (`PrimitiveComponent.SetSimulatePhysics` (`/Game/PuzzleBox/DavidKingsley/Core/BP_PushBlock_DK.PushBlock` _asbp_push_block_dk) false)
    (bind _output_get (set `self.Align` (+ (`self.Align`) 1)))
    (`KismetSystemLibrary.PrintString` "Set")
    (`KismetSystemLibrary.PrintString` (`KismetStringLibrary.Conv_IntToString` _output_get))
    (set `self.Overlapping18` false)))

(event `self.TriggerBox19.OnComponentBeginOverlap`
  (params (OverlappedComponent :type "PrimitiveComponent Object Reference") (OtherActor :type "Actor Object Reference") (OtherComp :type "PrimitiveComponent Object Reference") (OtherBodyIndex :type Integer) (bFromSweep :type Boolean) (SweepResult :type "HitResult Structure (by ref)"))
  ;[1 1 1] Box Trigger/ Counter 19
  (if (`self.Overlapping19`)
    (bind _asbp_push_block_dk (cast `/Game/PuzzleBox/DavidKingsley/Core/BP_PushBlock_DK` OtherActor))
    (`PrimitiveComponent.SetSimulatePhysics` (`/Game/PuzzleBox/DavidKingsley/Core/BP_PushBlock_DK.PushBlock` _asbp_push_block_dk) false)
    (bind _output_get (set `self.Align` (+ (`self.Align`) 1)))
    (`KismetSystemLibrary.PrintString` "Set")
    (`KismetSystemLibrary.PrintString` (`KismetStringLibrary.Conv_IntToString` _output_get))
    (set `self.Overlapping19` false)))

(event `self.TriggerBox4.OnComponentBeginOverlap`
  (params (OverlappedComponent :type "PrimitiveComponent Object Reference") (OtherActor :type "Actor Object Reference") (OtherComp :type "PrimitiveComponent Object Reference") (OtherBodyIndex :type Integer) (bFromSweep :type Boolean) (SweepResult :type "HitResult Structure (by ref)"))
  (if (`self.Overlapping4`)
    (bind _asbp_push_block_dk (cast `/Game/PuzzleBox/DavidKingsley/Core/BP_PushBlock_DK` OtherActor))
    (`PrimitiveComponent.SetSimulatePhysics` (`/Game/PuzzleBox/DavidKingsley/Core/BP_PushBlock_DK.PushBlock` _asbp_push_block_dk) false)
    (bind _output_get (set `self.Align` (+ (`self.Align`) 1)))
    (`KismetSystemLibrary.PrintString` "Hello")
    (`KismetSystemLibrary.PrintString` (`KismetStringLibrary.Conv_IntToString` _output_get))
    (set `self.Overlapping4` false)))

(fn `UserConstructionScript`)