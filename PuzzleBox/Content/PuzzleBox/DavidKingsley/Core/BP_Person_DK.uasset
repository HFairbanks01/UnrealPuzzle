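; BP_Person_DK is a player-controlled character for PuzzleBox that moves, jumps, looks vertically and shoots.
; Input axes drive movement along the actor's forward and right vectors and controller pitch, with no yaw input in this graph.
; Fire spawns a half-scale BP_Bullet_DK at the capsule's location and rotation.
; Any hit event on the capsule destroys the character, with no filter on what it hit.
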(event `self.ReceiveBeginPlay`)

(event `InputAction|Jump`
  (params (Key :type "Key Structure"))
  (:`Pressed`
    (`self.Jump`)))

(event `InputAxis|MoveHorizontal`
  (params (AxisValue :type "Float (single-precision)"))
  (`self.AddMovementInput` (`self.GetActorRightVector`) AxisValue))

(event `InputAxis|MoveZaxis`
  (params (AxisValue :type "Float (single-precision)"))
  (`self.AddMovementInput` (`self.GetActorForwardVector`) AxisValue))

(event `InputAction|Fire`
  (params (Key :type "Key Structure"))
  (bind (_returnvalue_location _returnvalue_rotation) (`KismetMathLibrary.BreakTransform` (`SceneComponent.K2_GetComponentToWorld` (`self.CapsuleComponent`))))
  (:`Pressed`
    (`|SpawnActorFromClass` "/Game/PuzzleBox/DavidKingsley/Core/BP_Bullet_DK.BP_Bullet_DK_C" (`KismetMathLibrary.MakeTransform` _returnvalue_location _returnvalue_rotation (0.5 0.5 0.5)) "Undefined" "OverrideRootScale" null null)))

(event `InputAxis|LookV`
  (params (AxisValue :type "Float (single-precision)"))
  (`self.AddControllerPitchInput` AxisValue))

(event `self.CapsuleComponent.OnComponentHit`
  (params (HitComponent :type "PrimitiveComponent Object Reference") (OtherActor :type "Actor Object Reference") (OtherComp :type "PrimitiveComponent Object Reference") (NormalImpulse :type "Vector Structure") (Hit :type "HitResult Structure (by ref)"))
  (`self.K2_DestroyActor`))

(fn `UserConstructionScript`)